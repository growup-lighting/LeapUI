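; Leap Motion test actor that recognises two-handed roll and horizontal swipe gestures, printing their names as debug text.
; Hand-moved events store each hand's Direction.Y, which swipe events compare, alongside a ±0.8 threshold, against gesture Direction.X for roll push/pull and Direction.Y for left/right swipes.
; Tick reports a roll when hands push and pull oppositely, then clears the flags every frame, so both swipes must land between ticks.
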(event EventSwipeGestureDetected
  (params (gesture :type Leap%20Swipe%20Gesture%20Object%20Reference))
  (bind _direction (Variables|/Script/LeapMotion.LeapSwipeGesture|GetDirection gesture))
  (bind _direction_2 (Variables|/Script/LeapMotion.LeapSwipeGesture|GetDirection gesture))
  (bind _x (Math|Vector|BreakVector _direction_2))
  (bind _x_2 (Math|Vector|BreakVector _direction_2))
  (bind _x_3 (Math|Vector|BreakVector _direction_2))
  (bind _y (Math|Vector|BreakVector _direction))
  (bind _y_2 (Math|Vector|BreakVector _direction))
  (bind _y_3 (Math|Vector|BreakVector _direction))
  (bind _y_4 (Math|Vector|BreakVector _direction))
  (bind _x_4 (Math|Vector|BreakVector _direction_2))
  (Utilities|FlowControl|Sequence ; 0:Roll,1:Swipe_Horizontal
    (:then_0
      ;[1 1 1] ロールイベントの取得
      (bind _returnvalue (Class|LeapSwipeGesture|Pointable gesture))
      (bind _returnvalue_2 (Class|LeapPointable|Hand _returnvalue))
      (Utilities|FlowControl|Sequence
        (:then_0
          (if (Math|Boolean|ANDBoolean (Variables|/Script/LeapMotion.LeapHand|GetIsRight _returnvalue_2) (>= _x_3 (Variables|Default|GetRightHandPosition)) (>= _x_3 0.8))
            (Variables|Default|SetRightRollPush true)))
        (:then_1
          (if (Math|Boolean|ANDBoolean (Variables|/Script/LeapMotion.LeapHand|GetIsRight _returnvalue_2) (<= _x_4 (Variables|Default|GetRightHandPosition)) (<= _x_4 -0.8))
            (Variables|Default|SetRightRollPull true)))
        (:then_2
          (if (Math|Boolean|ANDBoolean (Variables|/Script/LeapMotion.LeapHand|GetIsLeft _returnvalue_2) (>= _x (Variables|Default|GetleftHandPosition)) (>= _x 0.8))
            (Variables|Default|SetLeftRollPush true)))
        (:then_3
          (if (Math|Boolean|ANDBoolean (Variables|/Script/LeapMotion.LeapHand|GetIsLeft _returnvalue_2) (<= _x_2 (Variables|Default|GetleftHandPosition)) (<= _x_2 -0.8))
            (Variables|Default|SetLeftRollPull true)))))
    (:then_1
      ;[1 1 1] 水平スワイプイベントの取得
      (bind _returnvalue_3 (Class|LeapSwipeGesture|Pointable gesture))
      (bind _returnvalue_4 (Class|LeapPointable|Hand _returnvalue_3))
      (Utilities|FlowControl|Sequence
        (:then_0
          (if (Math|Boolean|ANDBoolean (Variables|/Script/LeapMotion.LeapHand|GetIsRight _returnvalue_4) (>= _y (Variables|Default|GetRightHandPosition)) (>= _y 0.8))
            (Development|PrintString "RightHandRight")))
        (:then_1
          (if (Math|Boolean|ANDBoolean (Variables|/Script/LeapMotion.LeapHand|GetIsRight _returnvalue_4) (<= _y_2 (Variables|Default|GetRightHandPosition)) (<= _y_2 -0.8))
            (Development|PrintString "RightHandLeft")))
        (:then_2
          (if (Math|Boolean|ANDBoolean (Variables|/Script/LeapMotion.LeapHand|GetIsLeft _returnvalue_4) (>= _y_3 (Variables|Default|GetLeftHandPosition)) (>= _y_3 0.8))
            (Development|PrintString "LeftHandRight")))
        (:then_3
          (if (Math|Boolean|ANDBoolean (Variables|/Script/LeapMotion.LeapHand|GetIsLeft _returnvalue_4) (<= _y_4 (Variables|Default|GetLeftHandPosition)) (<= _y_4 -0.8))
            (Development|PrintString "LeftHandLeft")))))))

(event EventLeapRightHandMoved
  (params (hand :type Leap%20Hand%20Object%20Reference))
  ;[1 1 1] 右手のポジションを取得
  (Variables|Default|SetRightHandPosition (.Y (Math|Vector|BreakVector (Variables|/Script/LeapMotion.LeapHand|GetDirection hand))))
  (Variables|Default|SetRightHand true))

(event EventLeapLeftHandMoved
  (params (hand :type Leap%20Hand%20Object%20Reference))
  ;[1 1 1] 左手のポジションを取得
  (Variables|Default|SetLeftHandPosition (.Y (Math|Vector|BreakVector (Variables|/Script/LeapMotion.LeapHand|GetDirection hand))))
  (Variables|Default|SetLeftHand true))

(event EventTick
  (params (DeltaSeconds :type Float%20%28single-precision%29))
  (if (and (Variables|Default|GetRightRollPull) (Variables|Default|GetLeftRollPush))
    (Development|PrintString "RightRoll")
    (Variables|Default|SetRightRollPull false)
    (Variables|Default|SetLeftRollPull false)
    (Variables|Default|SetLeftRollPush false)
    (Variables|Default|SetRightRollPush false)
    (Variables|Default|SetRightHand false)
    (Variables|Default|SetLeftHand false)
    (elif (and (Variables|Default|GetRightRollPush) (Variables|Default|GetLeftRollPull))
      (Development|PrintString "LeftRoll")
      (Variables|Default|SetRightRollPull false)
      (Variables|Default|SetLeftRollPull false)
      (Variables|Default|SetLeftRollPush false)
      (Variables|Default|SetRightRollPush false)
      (else
        (Variables|Default|SetRightRollPull false)
        (Variables|Default|SetLeftRollPull false)
        (Variables|Default|SetLeftRollPush false)
        (Variables|Default|SetRightRollPush false)))))

(event EventBeginPlay
  ;[1 1 1] SwipeGestureの有効
  (Class|LeapController|EnableGesture (Variables|Default|GetLeapController) "GESTURE_TYPE_SWIPE" true))

(event EventActorBeginOverlap
  (params (OtherActor :type Actor%20Object%20Reference)))

(event EventTick
  (params (DeltaSeconds :type Float%20%28single-precision%29)))

(fn ConstructionScript)